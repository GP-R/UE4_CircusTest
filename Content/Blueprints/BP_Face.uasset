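; BP_Face is an interactable actor with a Cube mesh that highlights and launches a cutscene-style Level Sequence.
; StartHighlight and EndHighlight switch the highlight on and off through the "Highlight" scalar parameter on the cube's materials.
; Interaction creates a Level Sequence player for Scene_1_01 and plays it.
; Event graph and construction script are empty, so all behavior depends on outside calls to these three functions.
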(event `self.ReceiveTick`
  (params (DeltaSeconds :type "Float (single-precision)")))

(fn `EndHighlight`
  (`MeshComponent.SetScalarParameterValueOnMaterials` (`self.Cube`) "Highlight" 0.0))

(fn `Interaction`
  (bind (_outactor _returnvalue) (`LevelSequencePlayer.CreateLevelSequencePlayer` "/Game/Cinematics/Takes/2023-01-07/Scene_1_01.Scene_1_01"))
  (`MovieSceneSequencePlayer.Play` _returnvalue))

(fn `StartHighlight`
  (params (HitActor :type "Actor Object Reference"))
  (`MeshComponent.SetScalarParameterValueOnMaterials` (`self.Cube`) "Highlight" 1000.0))

(fn `UserConstructionScript`)