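; BP_Ladder is an interactable ladder actor that teleports the player instead of simulating climbing.
; StartHighlight and EndHighlight swap the Cube's material between yellow and red.
; Interaction moves player pawn 0 to a hardcoded world location without sweep, so the destination does not depend on the ladder's placement.
; A second teleport to a lower point is left unconnected and never runs, and the event graph is empty.
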(event `self.ReceiveTick`
  (params (DeltaSeconds :type "Float (single-precision)")))

(fn `EndHighlight`
  (`PrimitiveComponent.SetMaterial` (`self.Cube`) 0 "/Game/Blueprints/M_Red.M_Red"))

(fn `Interaction`
  (`self.K2_SetActorLocation` (`GameplayStatics.GetPlayerPawn` 0) (1040.0 -700.0 622.0) false true))

(fn `StartHighlight`
  (params (HitActor :type "Actor Object Reference"))
  (`PrimitiveComponent.SetMaterial` (`self.Cube`) 0 "/Game/Blueprints/M_Yellow.M_Yellow"))

(fn `UserConstructionScript`
  (`parent.UserConstructionScript`))