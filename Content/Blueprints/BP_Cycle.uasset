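; BP_Cycle is a Blueprint that adjusts its own location based on the player pawn's tilt and height.
; On Tick, when player pawn 0 rolls past a threshold to either side while above a minimum height, it sets its location slightly below the pawn's.
; If BP_Cycle is itself that pawn, this lowers it a fixed step per frame, independent of delta time.
; BeginPlay, overlap and construction logic are empty.
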(event `self.ReceiveBeginPlay`)

(event `self.ReceiveTick`
  (params (DeltaSeconds :type "Float (single-precision)"))
  (bind _returnvalue_roll (`KismetMathLibrary.BreakRotator` (`self.K2_GetActorRotation` (`GameplayStatics.GetPlayerPawn` 0))))
  (bind (_returnvalue_x _returnvalue_y _returnvalue_z) (`KismetMathLibrary.BreakVector` (`self.K2_GetActorLocation` (`GameplayStatics.GetPlayerPawn` 0))))
  (if (or (< _returnvalue_roll -30.0) (> _returnvalue_roll 30.0))
    (if (> _returnvalue_z 30.0)
      (`self.K2_SetActorLocation` (`KismetMathLibrary.MakeVector` _returnvalue_x _returnvalue_y (- _returnvalue_z 6.0))))))

(fn `UserConstructionScript`)